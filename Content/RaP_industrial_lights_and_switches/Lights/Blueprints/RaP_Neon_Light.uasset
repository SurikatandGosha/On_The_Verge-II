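; Neon light fixture with configurable on/off state, colors and brightness, plus optional flicker and destructibility.
; OnOFF drives the point light and emissive dynamic material from the construction script and every Tick.
; With Flicker enabled, Tick also recreates the material instance and restarts a Timeline that modulates intensity and emissive brightness.
; When Destroyable, first damage hides mesh and light, shows the destroyed component, and triggers sparks and sound.
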(event EventTick
  (params (DeltaSeconds :type Float%20%28single-precision%29))
  (Utilities|FlowControl|Sequence
    (:then_0
      (CallFunction|On/OFF))
    (:then_1
      ;[1 1 1] Flicker
      (if (Variables|Default|GetFlicker_?)
        (bind _returnvalue (Rendering|Material|CreateDynamicMaterialInstance (Variables|Default|GetStaticMesh) 1 "/Game/RaP_industrial_lights_and_switches/Lights/Materials/Emissive_Inst.Emissive_Inst" :!class /Script/Engine.PrimitiveComponent))
        (bind _output_get (Variables|Default|SetEmissive_brightness _returnvalue))
        (Variables|Default|Setemissive_color _output_get)
        (Rendering|Components|Light|SetIntensity (Variables|Default|GetPointLight) 0.0)
        (bind _newtrack_0 (Timeline|Timeline_0 PlayFromStart) ; Timeline curve is used to make the light and material emissive flicker
          (:Update
            (Rendering|Material|SetScalarParameterValue (Variables|Default|GetEmissive_brightness) "Emissive_brightness" (+ (* _newtrack_0 0.1) 0.001) :!class /Script/Engine.MaterialInstanceDynamic)
            (Rendering|Components|Light|SetIntensity (Variables|Default|GetPointLight) _newtrack_0)
            (Rendering|Material|SetVectorParameterValue (Variables|Default|Getemissive_color) "emissive_color" (Variables|Default|GetColor_Material_Emissive) :!class /Script/Engine.MaterialInstanceDynamic)))))))

(event Game|Damage|EventAnyDamage
  (params (Damage :type Float%20%28single-precision%29) (DamageType :type Damage%20Type%20Object%20Reference) (InstigatedBy :type Controller%20Object%20Reference) (DamageCauser :type Actor%20Object%20Reference))
  ;[1 1 1] Damage
  (if (Variables|Default|GetDestroyable_?)
    (Utilities|FlowControl|DoOnce false
      (:Completed
        (Audio|Components|Audio|Play (Variables|Default|GetReflections_Spark_Cue) 0.0)
        (Rendering|SetVisibility (Variables|Default|GetStaticMesh) false false)
        (Rendering|SetVisibility (Variables|Default|GetRaP_Neon_Ligh_Destroyed) true false)
        (Components|Activation|Activate (Variables|Default|GetP_SparkBurst) false)
        (Rendering|SetVisibility (Variables|Default|GetPointLight) false false)))))

(fn ConstructionScript
  (bind _returnvalue (Rendering|Material|CreateDynamicMaterialInstance (Variables|Default|GetStaticMesh) 1 0 :!class /Script/Engine.PrimitiveComponent))
  (bind _output_get (Variables|Default|SetEmissive_Color _returnvalue))
  (Variables|Default|SetEmissive_Brightness _output_get)
  (CallFunction|On/OFF))

(fn On/OFF
  (bind _pointlight (Variables|Default|GetPointLight))
  (bind _pointlight_2 (Variables|Default|GetPointLight))
  (if (Variables|Default|GetON/OFF_?)
    (Rendering|Components|Light|SetIntensity _pointlight_2 (Variables|Default|GetBrightness_Light))
    (Rendering|Components|Light|SetLightColor _pointlight_2 (Variables|Default|GetColor_Light) true)
    (Rendering|Material|SetVectorParameterValue (Variables|Default|GetEmissive_Color) "emissive_color" (Variables|Default|GetColor_Material_Emissive) :!class /Script/Engine.MaterialInstanceDynamic)
    (Rendering|Material|SetScalarParameterValue (Variables|Default|GetEmissive_Brightness) "Emissive_brightness" (Variables|Default|GetBrightness_Emissive) :!class /Script/Engine.MaterialInstanceDynamic)
    (else
      (Rendering|Components|Light|SetIntensity _pointlight 0.0)
      (Rendering|Components|Light|SetLightColor :self _pointlight)
      (Rendering|Material|SetVectorParameterValue (Variables|Default|GetEmissive_Color) "emissive_color" "(R=0.510000,G=0.510000,B=0.510000,A=1.000000)" :!class /Script/Engine.MaterialInstanceDynamic)
      (Rendering|Material|SetScalarParameterValue (Variables|Default|GetEmissive_Brightness) "Emissive_brightness" 0.25 :!class /Script/Engine.MaterialInstanceDynamic)))
  (return))